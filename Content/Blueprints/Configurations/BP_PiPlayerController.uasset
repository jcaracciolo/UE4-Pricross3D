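; Player controller that lets the player rotate a BP_PiPuzzle actor by clicking and dragging with the mouse.
; Left press traces under the cursor against WorldDynamic objects and stores a hit puzzle, and release clears it.
; While a puzzle is held, mouse X and Y axes apply inverted, scaled world-space yaw and pitch to its root component.
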(event `Key|LeftMouseButton`
  (params (Key :type "Key Structure"))
  (bind (_hitresult _returnvalue) (`self.GetHitResultUnderCursorForObjects` (`GameplayStatics.GetPlayerController` 0) (`|MakeArray` "ObjectTypeQuery2" :!type "EObjectTypeQuery Enum") true))
  (:`Pressed`
    (if _returnvalue
      (bind _asbp_pi_puzzle (cast `/Game/Blueprints/GameLogic/BP_PiPuzzle` (`.HitActor` (`GameplayStatics.BreakHitResult` _hitresult))))
      (set `self.Puzzle` _asbp_pi_puzzle)))
  (:`Released`
    (set `self.Puzzle` null)))

(event `InputAxisKey|MouseX`
  (params (AxisValue :type "Float (single-precision)"))
  (bind _puzzle (`self.Puzzle`))
  (`/Engine/EditorBlueprintResources/StandardMacros.IsValid` _puzzle
    (:`Is Valid`
      (`SceneComponent.K2_AddWorldRotation` (`Actor.RootComponent` _puzzle) (`KismetMathLibrary.MakeRotator` 0.0 0.0 (* AxisValue -5.0)) false false))))

(event `InputAxisKey|MouseY`
  (params (AxisValue :type "Float (single-precision)"))
  (bind _puzzle (`self.Puzzle`))
  (`/Engine/EditorBlueprintResources/StandardMacros.IsValid` _puzzle
    (:`Is Valid`
      (`SceneComponent.K2_AddWorldRotation` (`Actor.RootComponent` _puzzle) (`KismetMathLibrary.MakeRotator` 0.0 (* AxisValue -5.0)) false false))))

(fn `UserConstructionScript`)