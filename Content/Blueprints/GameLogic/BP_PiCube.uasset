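; BP_PiCube is a puzzle cube that displays number hints per axis and can be toggled between painted and unpainted, apparently for a 3D Picross-style puzzle.
; Axis hint events extend their parent versions and use SetHint to write the number on two text components, also updating their circle and square markers.
; TogglePaint swaps the outline material to match IsPainted.
; SetSolutionColor hides all hints and applies the solution material.
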(event `self.SetXHint`
  (params (Hint :type "Hint Structure"))
  ;[1 1 1] Set Number Value on Hints
  (`parent.SetXHint` Hint)
  (`self.SetHint` Hint (`self.TextX1`) (`self.CircleX1`) (`self.SquareX1`))
  (`self.SetHint` Hint (`self.TextX2`) (`self.CircleX2`) (`self.SquareX2`)))

(event `self.SetYHint`
  (params (Hint :type "Hint Structure"))
  ;[1 1 1] Set Number Value on Hints
  (`parent.SetYHint` Hint)
  (`self.SetHint` Hint (`self.TextY1`) (`self.CircleY1`) (`self.SquareY1`))
  (`self.SetHint` Hint (`self.TextY2`) (`self.CircleY2`) (`self.SquareY2`)))

(event `self.TogglePaint`
  (bind _cube (`self.Cube`))
  ;[1 1 1] Set Material to Painted / NotPainted
  (`parent.TogglePaint`)
  (if (`self.bIsPainted`)
    (`PrimitiveComponent.SetMaterial` _cube 0 "/Game/Blueprints/Materials/M_Cube_Outline_RedInst.M_Cube_Outline_RedInst")
    (else
      (`PrimitiveComponent.SetMaterial` _cube 0 "/Game/Blueprints/Materials/M_Cube_Outline_Inst.M_Cube_Outline_Inst"))))

(event `self.SetZHint`
  (params (Hint :type "Hint Structure"))
  ;[1 1 1] Set Number Value on Hints
  (`parent.SetZHint` Hint)
  (`self.SetHint` Hint (`self.TextZ1`) (`self.CircleZ1`) (`self.SquareZ1`))
  (`self.SetHint` Hint (`self.TextZ2`) (`self.CircleZ2`) (`self.SquareZ2`)))

(event `self.SetSolutionColor`
  (`SceneComponent.SetHiddenInGame` (`self.HintComponent`) true true)
  (`PrimitiveComponent.SetMaterial` (`self.Cube`) 0 (`self.SolutionMaterial`)))

(fn `UserConstructionScript`)